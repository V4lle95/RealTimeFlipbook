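; Runtime flipbook baker that renders a rotating static mesh into frames on a render target and exports it.
; A SceneCapture2D in show-only mode captures just the mesh and cube, and BeginPlay opens a canvas on the FlipBook target.
; Each NextFrame event rotates the mesh one step and draws the capture into the next column; row advancement is disconnected.
; A limit check closes the canvas, and Render exports the sheet.
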(event Custom|Next%20Frame%20>>
  (bind _flip_res (Variables|Default|GetFlip%20Res))
  (Utilities|FlowControl|Sequence
    (:then_0
      (if (not (>= (Variables|Default|GetNumber%20of%20TImes) (+ (Variables|Default|GetMax%20times) 1.0)))
        (if (>= (Variables|Default|GetNumber%20of%20TImes) (Variables|Default|GetMax%20times))
          (Rendering|EndDrawCanvastoRenderTarget (Variables|Default|GetContext) :!label _label)
          (else
            (Utilities|FlowControl|Sequence
              (:then_0
                (Transformation|AddWorldRotation (Variables|Default|GetStaticMesh) (Variables|Default|GetNew%20Rotation) false false))
              (:then_1
                (if (>= (Variables|Default|GetFlip%20Count%20Current%20) (+ (Variables|Default|GetFlip%20Count%20Max) 4.0))
                  (goto _label)
                  (else
                    (Variables|Default|SetCurrent%20Column (Math|Float|%(Float) (Variables|Default|GetFlip%20Count%20Current%20) (Variables|Default|GetFlip%20Count%20per%20Row%20)))
                    (Canvas|DrawTexture :self (Variables|Default|GetCanvas) :RenderTexture (Variables|Default|GetCapture%20) :ScreenPosition (Math|Vector2D|MakeVector2D (* (Variables|Default|GetCurrent%20Column) (Variables|Default|GetFlip%20Res)) (* (Variables|Default|GetCurrent%20Row) (Variables|Default|GetFlip%20Res))) :ScreenSize (Math|Vector2D|MakeVector2D _flip_res _flip_res) :CoordinateSize "(X=1.000000,Y=1.000000)" :RenderColor (Utilities|Struct|MakeLinearColor 1.0 1.0 1.0 1.0) :BlendMode "BLEND_Opaque" :PivotPoint "(X=0.500000,Y=0.500000)")
                    (Math|Float|IncrementFloat (Variables|Default|GetFlip%20Count%20Current%20)
                      (:%20%20
                        (Math|Float|IncrementFloat (Variables|Default|GetNumber%20of%20TImes))))))))))))
    (:then_1
      (Development|PrintString (Utilities|String|Append (Utilities|String|ToString(Float) (Variables|Default|GetNumber%20of%20TImes)) " 
" (Utilities|String|ToString(Rotator) (Variables|Default|GetNew%20Rotation)))))))

(event Custom|Render
  (Rendering|ExportRenderTarget (Variables|Default|GetFlipBook) (Variables|Default|GetFile%20Path) (Variables|Default|GetFile%20Name)))

(event EventBeginPlay
  (bind _scenecapturecomponent2d (Variables|Default|GetSceneCaptureComponent2D))
  (bind _flipbook (Variables|Default|GetFlipBook))
  (bind _rotaton_object (Variables|Default|GetRotaton%20Object))
  (bind _max_times (Variables|Default|GetMax%20times))
  (Transformation|SetWorldRotation (Variables|Default|GetStaticMesh) "0, 0, 0" false false)
  (Variables|Default|SetNew%20Rotation (Math|Rotator|MakeRotator (/ (.roll _rotaton_object) _max_times) (/ (.pitch _rotaton_object) _max_times) (/ (.yaw _rotaton_object) _max_times)))
  (Rendering|SceneCapture|ClearShowOnlyComponents _scenecapturecomponent2d)
  (Class|SceneCaptureComponent|ClearHiddenComponents _scenecapturecomponent2d)
  (Utilities|Array|Clear (Variables|/Script/Engine.SceneCaptureComponent|GetShowOnlyActors _scenecapturecomponent2d))
  (Rendering|SceneCapture|ShowOnlyComponent _scenecapturecomponent2d (Variables|Default|GetStaticMesh))
  (Rendering|SceneCapture|ShowOnlyComponent _scenecapturecomponent2d (Variables|Default|GetCube))
  (Variables|/Script/Engine.SceneCaptureComponent|SetPrimitiveRenderMode _scenecapturecomponent2d "PRM_UseShowOnlyList")
  (Variables|/Script/Engine.SceneCaptureComponent2D|SetbConsiderUnrenderedOpaquePixelAsFullyTranslucent _scenecapturecomponent2d true)
  (Rendering|ClearRenderTarget2D _flipbook "(R=0.000000,G=0.000000,B=0.000000,A=0.000000)")
  (bind (_canvas _size _context) (Rendering|BeginDrawCanvastoRenderTarget _flipbook))
  (Variables|Default|SetCanvas _canvas)
  (Variables|Default|SetRes%20RT _size)
  (Variables|Default|SetContext _context)
  (bind _output_get (Variables|Default|SetFlip%20Count%20per%20Row%20 (/ (.x (Variables|Default|GetRes%20RT)) (Variables|Default|GetFlip%20Res))))
  (Variables|Default|SetFlip%20Count%20Max (* _output_get _output_get))
  (Variables|Default|SetNumber%20of%20TImes 0.0))

(event EventTick
  (params (DeltaSeconds :type Float%20%28single-precision%29)))

(fn ConstructionScript
  (bind _rotaton_object (Variables|Default|GetRotaton%20Object))
  (bind _max_times (Variables|Default|GetMax%20times))
  (Transformation|SetWorldRotation (Variables|Default|GetStaticMesh) "0, 0, 0" false false)
  (Variables|Default|SetNew%20Rotation (Math|Rotator|MakeRotator (/ (.roll _rotaton_object) _max_times) (/ (.pitch _rotaton_object) _max_times) (/ (.yaw _rotaton_object) _max_times))))